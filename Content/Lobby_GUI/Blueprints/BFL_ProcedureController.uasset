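; Blueprint function library for the lobby GUI that spawns popup widgets: dialogs, toast messages and choice screens.
; Each function creates its widget for player 0 with the passed parameters, adds it to the viewport, opens it and returns it.
; OpenDialog takes the widget class as input, while ShowToast and OpenChoice use W_Toast and W_Choice.
; Each also binds handlers to the widget's close and, where used, confirm or cancel events.
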(fn `OpenChoice`
  (params (CardType :type "/Game/Paperland_DataTables/Card_Data/E_CardType Enum" :default "NewEnumerator0"))
  (returns (Widget :type "/Game/Paperland_Blueprints/Cards/W_Choice Object Reference"))
  (bind _returnvalue (`|CreateWidget` "/Game/Paperland_Blueprints/Cards/W_Choice.W_Choice_C" (`GameplayStatics.GetPlayerController` null) CardType))
  (`UserWidget.AddToViewport` _returnvalue 0)
  (`/Game/Lobby_GUI/Blueprints/BPI_Dialog.Open` _returnvalue)
  (add `/Game/Paperland_Blueprints/Cards/W_Choice.OnCanceled` _returnvalue (`|CreateDelegate` _returnvalue :!event `Close`))
  (add `/Game/Paperland_Blueprints/Cards/W_Choice.OnClosed` _returnvalue (`|CreateDelegate` _returnvalue :!event `RemoveFromParent`))
  (return _returnvalue))

(fn `OpenDialog`
  (params (Dialog :type "/Game/Lobby_GUI/Blueprints/W_Dialog Class Reference") (Title :type Text) (Confirm :type Text :default "NSLOCTEXT(\"[C91CB1C0C66172D9A21EF599F1B3B215]\", \"2C7685D046239835F58D90A136A38EFC\", \"确认\")") (Cancel :type Text :default "NSLOCTEXT(\"[C91CB1C0C66172D9A21EF599F1B3B215]\", \"3EBB3A60422DDC6E09A805ACD8C38647\", \"取消\")") (TextLines :type "Array of Text"))
  (returns (Widget :type "/Game/Lobby_GUI/Blueprints/W_Dialog Object Reference"))
  (bind _returnvalue (`|CreateWidget` Dialog (`GameplayStatics.GetPlayerController` null) Title Confirm TextLines Cancel))
  (`UserWidget.AddToViewport` _returnvalue 0)
  (`/Game/Lobby_GUI/Blueprints/BPI_Dialog.Open` _returnvalue)
  (add `/Game/Lobby_GUI/Blueprints/W_Dialog.OnConfirmed` _returnvalue (`|CreateDelegate` _returnvalue :!event `Close`))
  (add `/Game/Lobby_GUI/Blueprints/W_Dialog.OnCanceled` _returnvalue (`|CreateDelegate` _returnvalue :!event `Close`))
  (add `/Game/Lobby_GUI/Blueprints/W_Dialog.OnClosed` _returnvalue (`|CreateDelegate` _returnvalue :!event `RemoveFromParent`))
  (return _returnvalue))

(fn `ShowToast`
  (params (Text :type Text) (Duration :type "Float (double-precision)" :default 2.0))
  (returns (Toast :type "/Game/Lobby_GUI/Blueprints/W_Toast Object Reference"))
  (bind _returnvalue (`|CreateWidget` "/Game/Lobby_GUI/Blueprints/W_Toast.W_Toast_C" (`GameplayStatics.GetPlayerController` null) Text Duration))
  (`UserWidget.AddToViewport` _returnvalue 0)
  (message `/Game/Lobby_GUI/Blueprints/BPI_Dialog.Open` _returnvalue)
  (add `/Game/Lobby_GUI/Blueprints/W_Toast.OnClosed` _returnvalue (`|CreateDelegate` _returnvalue :!event `RemoveFromParent`))
  (return _returnvalue))