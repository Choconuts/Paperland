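; Card effect Blueprint that places a block on a sea hex of the hex map.
; It accepts only unoccupied sea hexes as valid selections.
; On selection it runs the parent handler, looks up BlockInfoName in a data table and asks HexMap to create that block at the hex's coordinate.
; It reports failure if the parent handler fails or the row is missing.
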(fn `HandleSelectionSeaHex`
  (params (SeaHex :type "Object Object Reference"))
  (returns (Handled :type Boolean))
  (bind _handled (`parent.HandleSelectionSeaHex` SeaHex))
  (if _handled
    (bind _returnvalue (`|GetDataTableRow` null (`self.BlockInfoName`))
      (:`then`
        (message `/Game/CardSystem/BP_BlockCardEffect.CreateBlock` (`.HexMap` (`self.HexMap`)) (`/Game/CardSystem/BP_BlockCardEffect.Coord` SeaHex) _returnvalue)
        (return true))
      (:`RowNotFound`
        _)))
  (return false))

(fn `UserConstructionScript`
  (`parent.UserConstructionScript`))

(fn `ValidateSelectionSeaHex`
  (params (SeaHex :type "Object Object Reference"))
  (returns (CanSelect :type Boolean) (Valid :type Boolean))
  (return true (not (`/Game/CardSystem/BP_BlockCardEffect.IsOccupied` SeaHex))))