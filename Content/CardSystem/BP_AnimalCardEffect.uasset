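; BP_AnimalCardEffect is the effect of an animal card, validating a selected hex block and sending the animal to the hex map via CreateAnimalMessage.
; Validation checks the block's animal slot and compares its type and six neighbors against the card's BlockTint pattern.
; The neighbor ring is tested in all six rotations, so orientation does not matter.
; Tints match by substring, with "None" acting as a wildcard that also accepts missing blocks.
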(fn `CheckEnvironmentMatched`
  (params (Block :type "Object Object Reference"))
  (returns (Matched :type Boolean))
  (locals (IsMatched :type Boolean :default false))
  (bind _coord (`/Game/CardSystem/BP_AnimalCardEffect.Coord` Block))
  (bind (_isanimal _blocktint) (break `/Game/CardSystem/S_AnimalInfo` (`.AnimalInfo_16_69D07F894D33860BFA4E0D9AA80D70F6` (break `/Game/Demo/S_CardInfo` (`self.CardInfo`)))))
  (if (and (`self.MatchBlock` (`|GetArrayItem` _blocktint) _coord) _isanimal)
    (for _index (range 6)
      (bind _ismatched (`self.MatchPattern` _index (`self.GetNeighborCoords` _coord) _blocktint))
      (set `local.IsMatched` (or _ismatched (`local.IsMatched`))))
    (return (`local.IsMatched`))
    (else
      (return false))))

(fn `HandleSelectionBlock`
  (params (Block :type "Object Object Reference"))
  (returns (Handled :type Boolean))
  (bind _handled (`parent.HandleSelectionBlock` Block))
  (if _handled
    (message `/Game/CardSystem/BP_AnimalCardEffect.CreateAnimal` (`.HexMap` (`self.HexMap`)) (`/Game/CardSystem/BP_AnimalCardEffect.Coord` Block) (`.AnimalInfo_16_69D07F894D33860BFA4E0D9AA80D70F6` (break `/Game/Demo/S_CardInfo` (`self.CardInfo`))))
    (return true)
    (else
      (return false))))

(fn `MatchBlock`
  (params (BlockTint :type String) (Coord :type "IntVector Structure"))
  (returns (IsMatched :type Boolean))
  (bind (_value _returnvalue) (`BlueprintMapLibrary.Map_Find` (`/Game/CardSystem/BP_AnimalCardEffect.BlockMap` (`.HexMap` (`self.HexMap`))) (`local.Coord`)))
  (if _returnvalue
    (return (or (`KismetStringLibrary.Contains` (`local.BlockTint`) (`|GetEnumeratorNameAsString` (`.BlockType_3_BCD7B8E44A1F03E042087AB6AD4C69B6` (break `FallbackStruct` (`/Game/CardSystem/BP_AnimalCardEffect.BlockInfo` _value))))) (`KismetStringLibrary.Contains` (`local.BlockTint`))))
    (else
      (return (`KismetStringLibrary.Contains` (`local.BlockTint`))))))

(fn `MatchPattern`
  (params (StartIndex :type Integer) (NeighborCoords :type "Array of IntVector Structure") (BlockHints :type "Array of String"))
  (returns (IsMatched :type Boolean))
  (locals (LocalMatched :type Boolean :default true))
  (for _index (range 6)
    (set `local.LocalMatched` (and (`local.LocalMatched`) (`self.MatchBlock` (`|GetArrayItem` BlockHints (+ (mod (+ _index StartIndex) 6) 1)) (`|GetArrayItem` NeighborCoords _index)))))
  (return (`local.LocalMatched`)))

(fn `UserConstructionScript`
  (`parent.UserConstructionScript`))

(fn `ValidateSelectionBlock`
  (params (Block :type "Object Object Reference"))
  (returns (CanSelect :type Boolean) (Valid :type Boolean))
  (return true (and (`self.CheckEnvironmentMatched` Block) (== (`/Game/CardSystem/BP_AnimalCardEffect.Animal` Block) null))))