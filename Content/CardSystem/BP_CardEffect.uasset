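; Base actor for card effects that target sea hexes or blocks on the hex map during a cast.
; On BeginPlay it gets the HexMap from the player controller and binds to hover and click events.
; Hover highlights targets through validation functions that reject everything by default, apparently override points for child effects.
; A handled click sends FinishCastMessage, clears all selection marks and destroys the actor; CancelCast unbinds and destroys it.
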(event `self.ReceiveBeginPlay`
  (`self.InitializeBindings`
    (:`Success`
      (add `/Game/MapSystem/BP_HexMap.OnSeaHexInteractionHover` (`self.HexMap`) (delegate `OnSeaHover`))
      (add `/Game/MapSystem/BP_HexMap.OnSeaHexInteractionClick` (`self.HexMap`) (delegate `OnSeaClicked`))
      (`self.InitializeBindings`
        (:`Success`
          (add `/Game/MapSystem/BP_HexMap.OnBlockInteractionHover` (`self.HexMap`) (delegate `OnBlockHover`))
          (add `/Game/MapSystem/BP_HexMap.OnBlockInteractionClick` (`self.HexMap`) (delegate `OnBlockClick`)))))))

(event `OnSeaClicked`
  (params (SeaHex :type "/Game/MapSystem/BP_SeaHex Object Reference"))
  (bind _handled (`self.HandleSelectionSeaHex` SeaHex))
  (if _handled
    (remove `/Game/MapSystem/BP_HexMap.OnSeaHexInteractionHover` (`self.HexMap`) (delegate `OnSeaHover`))
    (remove `/Game/MapSystem/BP_HexMap.OnSeaHexInteractionClick` (`self.HexMap`) (delegate `OnSeaClicked`))
    (remove `/Game/MapSystem/BP_HexMap.OnSeaHexInteractionClick` (`self.HexMap`) (delegate `OnSeaClicked`))
    (message `/Game/CardSystem/BPI_CastCards.FinishCast` (`GameplayStatics.GetPlayerController` 0))
    (`self.ResetSelection`
      (:`out`
        (`self.K2_DestroyActor`)))))

(event `OnSeaHover`
  (params (IsEnter :type Boolean) (SeaHex :type "/Game/MapSystem/BP_SeaHex Object Reference"))
  (bind (_canselect _valid) (`self.ValidateSelectionSeaHex` SeaHex))
  (if IsEnter
    (`/Game/MapSystem/BP_SeaHex.MarkSelection` SeaHex _canselect _valid)
    (else
      (`/Game/MapSystem/BP_SeaHex.MarkSelection` SeaHex false false))))

(event `/Game/CardSystem/BPI_CastCards.CancelCast`
  (bind _hexmap (`self.HexMap`))
  (bind _hexmap_2 (`self.HexMap`))
  (remove `/Game/MapSystem/BP_HexMap.OnSeaHexInteractionHover` _hexmap_2 (delegate `OnSeaHover`))
  (remove `/Game/MapSystem/BP_HexMap.OnSeaHexInteractionClick` _hexmap_2 (delegate `OnSeaClicked`))
  (remove `/Game/MapSystem/BP_HexMap.OnBlockInteractionHover` _hexmap (delegate `OnBlockHover`))
  (remove `/Game/MapSystem/BP_HexMap.OnBlockInteractionClick` _hexmap (delegate `OnBlockClick`))
  (`self.K2_DestroyActor`))

(event `OnBlockClick`
  (params (Block :type "/Game/MapSystem/BP_HexBlock Object Reference"))
  (bind _hexmap (`self.HexMap`))
  (bind _handled (`self.HandleSelectionBlock` Block))
  (if _handled
    (remove `/Game/MapSystem/BP_HexMap.OnBlockInteractionHover` _hexmap (delegate `OnBlockHover`))
    (remove `/Game/MapSystem/BP_HexMap.OnBlockInteractionClick` _hexmap (delegate `OnBlockClick`))
    (message `/Game/CardSystem/BPI_CastCards.FinishCast` (`GameplayStatics.GetPlayerController` 0))
    (`self.ResetSelection`
      (:`out`
        (`self.K2_DestroyActor`)))))

(event `OnBlockHover`
  (params (Block :type "/Game/MapSystem/BP_HexBlock Object Reference") (Enter :type Boolean))
  (bind (_canselect _valid) (`self.ValidateSelectionBlock` Block))
  (if Enter
    (`/Game/CardSystem/BPI_CastCards.MarkSelection` Block _canselect _valid)
    (else
      (`/Game/CardSystem/BPI_CastCards.MarkSelection` Block false false))))

(fn `HandleSelectionBlock`
  (params (Block :type "/Game/MapSystem/BP_HexBlock Object Reference"))
  (returns (Handled :type Boolean))
  (bind (_canselect _valid) (`self.ValidateSelectionBlock` Block))
  (return (and _canselect _valid)))

(fn `HandleSelectionSeaHex`
  (params (SeaHex :type "/Game/MapSystem/BP_SeaHex Object Reference"))
  (returns (Handled :type Boolean))
  (bind (_canselect _valid) (`self.ValidateSelectionSeaHex` SeaHex))
  (return (and _canselect _valid)))

(fn `InitializeBindingsOld`
  (bind _asbp_hex_map_player_controller (cast `/Game/MapSystem/BP_HexMapPlayerController` (`GameplayStatics.GetPlayerController` 0)))
  (set `self.HexMap` (`/Game/MapSystem/BP_HexMapPlayerController.GetHexMap` _asbp_hex_map_player_controller)))

(fn `UserConstructionScript`)

(fn `ValidateSelectionBlock`
  (params (Block :type "/Game/MapSystem/BP_HexBlock Object Reference"))
  (returns (CanSelect :type Boolean) (Valid :type Boolean))
  (return false false))

(fn `ValidateSelectionSeaHex`
  (params (SeaHex :type "/Game/MapSystem/BP_SeaHex Object Reference"))
  (returns (CanSelect :type Boolean) (Valid :type Boolean))
  (return false false))