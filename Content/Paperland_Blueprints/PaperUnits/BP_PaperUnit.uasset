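; BP_PaperUnit is a Paper2D flipbook unit (soldier or building) that billboards toward the player camera every tick.
; Construction applies the flipbook from UnitInfo, and BeginPlay makes the sprite transparent white and offsets its shadow by unit type.
; A gated Tick interpolates sprite color toward the environment color, fading it in on spawn.
; The gate closes once the color matches, and StartChangeColor reopens it.
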(event `self.ReceiveBeginPlay`
  (`self.SpawnAnimation`)
  (`self.SetShadowOffset`))

(event `self.ReceiveTick`
  (params (DeltaSeconds :type "Float (single-precision)"))
  (`|ExecutionSequence`
    (:`then_0`
      (`/Engine/EditorBlueprintResources/StandardMacros.Gate` false :!label _label
        (:`Exit`
          (`self.UpdateColor` DeltaSeconds
            (:`Unchanged`
              (goto _label :!via `Close`))))))
    (:`then_1`
      (`self.SetLookAtRotation`))))

(event `StartChangeColor`
  (goto _label :!via `Open`))

(fn `SetLookAtRotation`
  (`self.K2_SetActorRotation` (`PlayerCameraManager.GetCameraRotation` (`GameplayStatics.GetPlayerCameraManager` 0)))
  (`self.K2_AddActorLocalRotation` (struct :`Yaw` 90.0)))

(fn `SetShadowOffset`
  (switch `/Game/Paperland_DataTables/Unit_Data/E_UnitType` (`.UnitType_18_69DA8AC141482C2D86704BA3364C6635` (break `/Game/Paperland_DataTables/Unit_Data/S_UnitInfo` (`self.UnitInfo`)))
    (:`NewEnumerator2`
      (`SceneComponent.K2_SetRelativeLocation` (`self.Shadow`) (-10.0 0.0 5.0) false false))
    (:`NewEnumerator3`
      (`SceneComponent.K2_SetRelativeLocation` (`self.Shadow`) (5.0 -20.0 25.0) false false))))

(fn `SpawnAnimation`
  (`PaperFlipbookComponent.SetSpriteColor` (`self.士兵_Flipbook`) (struct :`R` 1.0 :`G` 1.0 :`B` 1.0)))

(fn `UserConstructionScript`
  (`PaperFlipbookComponent.SetFlipbook` (`self.士兵_Flipbook`) (`.Flipbook_11_9DD829E94EF8430F9FCAB8A470DE0B34` (break `/Game/Paperland_DataTables/Unit_Data/S_UnitInfo` (`self.UnitInfo`)))))