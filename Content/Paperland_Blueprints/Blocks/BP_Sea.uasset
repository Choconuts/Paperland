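; BP_Sea procedurally builds the sea from randomly picked block actors when play begins.
; From each InitSeaBlocks coordinate, GenerateBlocks recursively spreads to neighboring coordinates up to a fixed depth.
; BlockMap prevents duplicate spawns, and a block reached at a shallower depth lowers its stored RecursionDepth and expands again.
; New blocks are placed at grid-derived world positions with a downward Z offset.
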(event `self.ReceiveBeginPlay`
  (for _array_element (`self.InitSeaBlocks`)
    (`self.GenerateBlocks` _array_element 0 6)))

(fn `CoordToTransform`
  (params (Coord :type "IntVector2 Structure"))
  (returns (Transform :type "Transform Structure"))
  (return (`KismetMathLibrary.MakeTransform` (+ (`/Game/Paperland_Blueprints/GridSystem/BFL_GridSystem.CoordToWorldPosition` (`local.Coord`) (`self.UnitScale`)) (0.0 0.0 -60.0)))))

(fn `GenerateBlocks`
  (params (Coord :type "IntVector2 Structure") (Depth :type Integer) (MaxDepth :type Integer))
  (if (not (>= Depth MaxDepth))
    (bind (_block _exist) (`self.SpawnOrGetBlock` Coord Depth (`/Game/Paperland_DataTables/BFL_Database.GetRandomBlock`)))
    (if (not _exist)
      (bind _newparam (`/Game/Paperland_Blueprints/GridSystem/BFL_GridSystem.GetNeighborCoordOffset`))
      (for _array_element _newparam
        (`self.GenerateBlocks` (`/Game/Paperland_Blueprints/GridSystem/BFL_GridSystem.OffsetCoord` _array_element (`local.Coord`)) (+ (`local.Depth`) 1) (`local.MaxDepth`))))))

(fn `SpawnBlock`
  (params (BlockInfo :type "/Game/Paperland_DataTables/Block_Data/S_BlockInfo Structure") (Coord :type "IntVector2 Structure") (Depth :type Integer))
  (returns (Block :type "/Game/Paperland_Blueprints/Blocks/BP_Block Object Reference"))
  (bind _returnvalue (`|SpawnActorFromClass` (`.Block_9_DC91E3CD466EA2992BB378A693657991` (break `/Game/Paperland_DataTables/Block_Data/S_BlockInfo` BlockInfo)) (`self.CoordToTransform` Coord) "Undefined" "MultiplyWithRoot" null (`local.Coord`) Depth (`local.BlockInfo`) null))
  (return _returnvalue))

(fn `SpawnOrGetBlock`
  (params (Coord :type "IntVector2 Structure") (Depth :type Integer) (BlockInfo :type "/Game/Paperland_DataTables/Block_Data/S_BlockInfo Structure"))
  (returns (Block :type "/Game/Paperland_Blueprints/Blocks/BP_Block Object Reference") (Exist :type Boolean))
  (bind _coord (`local.Coord`))
  (bind _depth (`local.Depth`))
  (bind (_value _returnvalue) (`BlueprintMapLibrary.Map_Find` (`self.BlockMap`) (`local.Coord`)))
  (if _returnvalue
    (if (< _depth (`/Game/Paperland_Blueprints/Blocks/BP_Block.RecursionDepth` _value))
      (set `/Game/Paperland_Blueprints/Blocks/BP_Block.RecursionDepth` _depth _value)
      (return _value false)
      (else
        (return _value true)))
    (else
      (bind _block (`self.SpawnBlock` BlockInfo _coord Depth))
      (`BlueprintMapLibrary.Map_Add` (`self.BlockMap`) _coord _block)
      (return _block false))))

(fn `UserConstructionScript`)