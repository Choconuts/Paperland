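; Wood terrain block for Paperland that varies its tree decoration at random each time play begins.
; After the parent BeginPlay, RandomDecoration uses random integer switches to hide one or two of its tree components, including their children.
; Two of the three main outcomes share a second roll that also hides either Tree or Tree1, while the third hides only Tree1.
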(event `self.ReceiveBeginPlay`
  (`parent.ReceiveBeginPlay`)
  (`self.RandomDecoration`))

(fn `RandomDecoration`
  (switch `int` (`KismetMathLibrary.RandomIntegerInRange` 0 2)
    (:`Default`
      (`SceneComponent.SetVisibility` (`self.Tree`) false true))
    (:`0`
      (`SceneComponent.SetVisibility` (`self.Tree4`) false true)
      (switch `int` (`KismetMathLibrary.RandomIntegerInRange` 0 1) :!label _label
        (:`Default`
          (`SceneComponent.SetVisibility` (`self.Tree`) false true))
        (:`0`
          (`SceneComponent.SetVisibility` (`self.Tree1`) false true))))
    (:`1`
      (`SceneComponent.SetVisibility` (`self.Tree2`) false true)
      (goto _label))
    (:`2`
      (`SceneComponent.SetVisibility` (`self.Tree1`) false true))))

(fn `UserConstructionScript`)