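; BP_SeaBlockMesh is a sea block that appears as a blue hexagonal dynamic mesh.
; Its AppendPolygons function builds the shape with AppendHexagon, using the block's Radius and a fixed height.
; Tick reapplies blue to the mesh materials' Color parameter every frame, after calling the parent Tick.
; Clicking the actor only prints a debug string.
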(event `self.ReceiveBeginPlay`
  (`parent.ReceiveBeginPlay`))

(event `self.ReceiveTick`
  (params (DeltaSeconds :type "Float (single-precision)"))
  (`parent.ReceiveTick` DeltaSeconds)
  (`MeshComponent.SetVectorParameterValueOnMaterials` (`self.DynamicMeshComponent`) "Color" (0.0 0.0 1.0)))

(event `self.ReceiveActorOnClicked`
  (params (ButtonPressed :type "Key Structure"))
  (`KismetSystemLibrary.PrintString` "Click"))

(fn `AppendPolygons`
  (params (TargetMesh :type "DynamicMesh Object Reference"))
  (returns (OutputTargetMesh :type "DynamicMesh Object Reference"))
  (bind _outputtargetmesh (`self.AppendHexagon` TargetMesh (struct) (`self.Radius`) 2.0))
  (return _outputtargetmesh))

(fn `UserConstructionScript`
  (`parent.UserConstructionScript`))