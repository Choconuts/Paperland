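; BP_BlockMesh is a Geometry Script generated-mesh actor for blocks, forcing an immediate rebuild at BeginPlay.
; The rebuild event calls AppendPolygons, which by default extrudes a hexagon, then cleans degenerate triangles and applies the Materials array.
; AppendHexagon extrudes a six-point circle path with a material ID.
; AppendPrism, uncalled here, revolves a vertex path at a random angular offset, and ClearMaterials empties the material set.
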(event `self.ReceiveBeginPlay`
  (`parent.ReceiveBeginPlay`)
  (`self.Rebuild`))

(event `self.ClearMaterials`
  ;[1 1 1] CLEAR MATERIALS
  (`KismetArrayLibrary.Array_Clear` (`self.Materials`))
  (`DynamicMeshComponent.ConfigureMaterialSet` (`self.DynamicMeshComponent`) (`self.Materials`) true)
  ;[1 1 1] Hexagon Generation
  (bind _outputtargetmesh (`self.AppendPolygons` (stale `self.OnRebuildGeneratedMesh` TargetMesh) :!label _label))
  ;[1 1 1] Apply Material
  (`self.CleanDegenerateTris` _outputtargetmesh)
  (`DynamicMeshComponent.ConfigureMaterialSet` (`self.DynamicMeshComponent`) (`self.Materials`) true))

(event `self.OnRebuildGeneratedMesh`
  (params (TargetMesh :type "DynamicMesh Object Reference"))
  ;[1 1 1] Hexagon Generation
  (`KismetSystemLibrary.PrintString` "Build")
  (goto _label))

(fn `AppendHexagon`
  (params (TargetMesh :type "DynamicMesh Object Reference") (Transform :type "Transform Structure") (Radius :type "Float (double-precision)") (Height :type "Float (double-precision)") (MateiralIndex :type Integer))
  (returns (OutputTargetMesh :type "DynamicMesh Object Reference"))
  (bind _returnvalue (`GeometryScriptLibrary_PolyPathFunctions.CreateCirclePath2D` (0.0 0.0) Radius 6))
  (bind _returnvalue_2 (`GeometryScriptLibrary_MeshPrimitiveFunctions.AppendSimpleExtrudePolygon` (`local.TargetMesh`) (make `GeometryScriptPrimitiveOptions` "PerFace" false "Uniform" MateiralIndex) (`local.Transform`) (`GeometryScriptLibrary_PolyPathFunctions.Conv_GeometryScriptPolyPathToArrayOfVector2D` _returnvalue) (`local.Height`) 0 true "Base" null))
  (return _returnvalue_2))

(fn `AppendPolygons`
  (params (TargetMesh :type "DynamicMesh Object Reference"))
  (returns (OutputTargetMesh :type "DynamicMesh Object Reference"))
  (bind _outputtargetmesh (`self.AppendHexagon` TargetMesh (struct) 100.0 50.0))
  (return _outputtargetmesh))

(fn `AppendPrism`
  (params (TargetMesh :type "DynamicMesh Object Reference") (Steps :type Integer :default 6) (VertexArray :type "Array of Vector2D Structure") (MaterialIndex :type Integer))
  (returns (OutputTargetMesh :type "DynamicMesh Object Reference"))
  (bind _returnvalue (`GeometryScriptLibrary_MeshPrimitiveFunctions.AppendRevolvePath` TargetMesh (make `GeometryScriptPrimitiveOptions` "PerFace") (struct) VertexArray (make `GeometryScriptRevolveOptions` 360.0 (* (`KismetMathLibrary.RandomFloat`) 360.0)) Steps true null))
  (return _returnvalue))

(fn `Rebuild`
  (`self.MarkForMeshRebuild` true))

(fn `UserConstructionScript`
  (`parent.UserConstructionScript`))