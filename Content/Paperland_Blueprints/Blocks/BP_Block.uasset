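; BP_Block is a Paperland map block with a sea hexagon and a grid coordinate, which spawns a random paper unit when play begins.
; SpawnUnit creates a scaled BP_PaperUnit from the unit info at a random XY offset around the SpawnRange component, keeping that component's height.
; Every tick it tints the sea hexagon's material by RecursionDepth, and clicking the block prints its coordinate for debugging.
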(event `self.ReceiveBeginPlay`
  (`self.SpawnUnit` (`/Game/Paperland_DataTables/BFL_Database.GetRandomUnit`)))

(event `self.ReceiveTick`
  (params (DeltaSeconds :type "Float (single-precision)"))
  (`self.UpdateSeaColor`))

(event `self.ReceiveActorOnClicked`
  (params (ButtonPressed :type "Key Structure"))
  (`KismetSystemLibrary.PrintString` (`KismetStringLibrary.Conv_IntVector2ToString` (`self.Coord`))))

(fn `GetSpawnPosition`
  (returns (Position :type "Vector Structure"))
  (bind _spawnrange (`self.SpawnRange`))
  (bind _returnvalue (`SceneComponent.K2_GetComponentLocation` _spawnrange))
  (return (`KismetMathLibrary.MakeVector` (.x (+ (* (* (`KismetMathLibrary.RandomUnitVector`) (`SceneComponent.K2_GetComponentScale` _spawnrange)) (`self.RangeRadius`)) _returnvalue)) (.y (+ (* (* (`KismetMathLibrary.RandomUnitVector`) (`SceneComponent.K2_GetComponentScale` _spawnrange)) (`self.RangeRadius`)) _returnvalue)) (.z _returnvalue))))

(fn `SpawnUnit`
  (params (UnitInfo :type "/Game/Paperland_DataTables/Unit_Data/S_UnitInfo Structure"))
  (returns (Unit :type "/Game/Paperland_Blueprints/PaperUnits/BP_PaperUnit Object Reference"))
  (bind _returnvalue (`|SpawnActorFromClass` "/Game/Paperland_Blueprints/PaperUnits/BP_PaperUnit.BP_PaperUnit_C" (`KismetMathLibrary.MakeTransform` (`self.GetSpawnPosition`) (struct) (`KismetMathLibrary.Conv_DoubleToVector` (`self.UnitScale`))) "Undefined" "MultiplyWithRoot" null UnitInfo null))
  (return _returnvalue))

(fn `UpdateSeaColor`
  (`MeshComponent.SetVectorParameterValueOnMaterials` (`self.SeaHexagon`) "Color" (* (`self.RecursionDepth`) (`KismetMathLibrary.MakeVector` 0.08 0.08 0.3))))

(fn `UserConstructionScript`)