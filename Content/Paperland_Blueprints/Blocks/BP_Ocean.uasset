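; BP_Ocean builds and owns the game's block grid, a sea with terrain blocks, stored in a coordinate-keyed map.
; On BeginPlay it recursively grows default blocks around configured sea sources to a depth limit, revisiting cells reached by shorter paths.
; Configured or requested terrain replaces existing blocks at their coordinates.
; Helper functions return neighbors and match block types or neighbor patterns across six rotations.
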(event `self.ReceiveBeginPlay`
  (`self.InitializeByConfig`))

(event `/Game/Paperland_Blueprints/Blocks/BPI_OceanInteraction.CreateTerrainBlock`
  (params (Coord :type "IntVector2 Structure") (BlockInfo :type "/Game/Paperland_DataTables/Block_Data/S_BlockInfo Structure"))
  (`self.SpawnTerrainBlock` Coord BlockInfo))

(fn `CheckBlockMatch`
  (params (Block :type "/Game/Paperland_Blueprints/Blocks/BP_Block Object Reference") (Match :type "/Game/Paperland_DataTables/Block_Data/S_BlockMatch Structure"))
  (returns (Valid :type Boolean))
  (bind (_matchtype _targetblocktype _patternmap) (break `/Game/Paperland_DataTables/Block_Data/S_BlockMatch` Match))
  (if (`self.CheckMatchBlockType` (`.BlockType_12_DB45E6C2411A13B30C8194B614184F99` (break `/Game/Paperland_DataTables/Block_Data/S_BlockInfo` (`/Game/Paperland_Blueprints/Blocks/BP_Block.BlockInfo` Block))) _targetblocktype)
    (switch `/Game/Paperland_DataTables/Block_Data/E_MatchType` _matchtype
      (:`NewEnumerator0`
        (return (`self.CheckBlockMatchPattern` Block _patternmap)))
      (:`NewEnumerator2`
        (return true))
      (:`NewEnumerator3`
        (return false)))
    (else
      (return false))))

(fn `CheckBlockMatchPattern`
  (params (Block :type "/Game/Paperland_Blueprints/Blocks/BP_Block Object Reference") (Pattern :type "Map of IntVector2 Structure to /Game/Paperland_DataTables/Block_Data/E_BlockType Enum"))
  (returns (NewParam :type Boolean))
  (locals (RotationAccepted :type Boolean))
  (if (`BlueprintMapLibrary.Map_IsEmpty` Pattern)
    (return false)
    (else
      (for _index (range 6)
        (set `local.RotationAccepted` true)
        (bind (_keypin _valuepin) (`|MapForEach` Pattern :!label _label)
          (:`then`
            (bind (_value _returnvalue) (`BlueprintMapLibrary.Map_Find` (`self.BlockMap`) (`/Game/Paperland_Blueprints/GridSystem/BFL_GridSystem.OffsetCoord` (`/Game/Paperland_Blueprints/Blocks/BP_Block.Coord` (`local.Block`)) (`/Game/Paperland_Blueprints/GridSystem/BFL_GridSystem.RotateOffset` _keypin _index))))
            (if _returnvalue
              (bind _output_get (set `local.RotationAccepted` (`self.CheckMatchBlockType` (`.BlockType_12_DB45E6C2411A13B30C8194B614184F99` (break `/Game/Paperland_DataTables/Block_Data/S_BlockInfo` (`/Game/Paperland_Blueprints/Blocks/BP_Block.BlockInfo` _value))) _valuepin)))
              (if (not _output_get)
                (goto _label :!via `BreakPin`))))
          (:`CompletedPin`
            (if (`local.RotationAccepted`)
              (return true)))))
      (return false))))

(fn `CheckMatchBlockType`
  (params (BlockType :type "/Game/Paperland_DataTables/Block_Data/E_BlockType Enum" :default "NewEnumerator0") (MatchType :type "/Game/Paperland_DataTables/Block_Data/E_BlockType Enum" :default "NewEnumerator0"))
  (returns (Valid :type Boolean))
  (if (`|EnumEquality` MatchType "NewEnumerator5")
    (return (`|EnumInequality` (`local.BlockType`) "NewEnumerator6"))
    (else
      (return (`|EnumEquality` (`local.BlockType`) (`local.MatchType`))))))

(fn `CoordToTransform`
  (params (Coord :type "IntVector2 Structure"))
  (returns (Transform :type "Transform Structure"))
  (return (`KismetMathLibrary.MakeTransform` (+ (`/Game/Paperland_Blueprints/GridSystem/BFL_GridSystem.CoordToWorldPosition` (`local.Coord`) (`self.UnitScale`)) (0.0 0.0 -60.0)))))

(fn `GenerateBlocks`
  (params (Coord :type "IntVector2 Structure") (Depth :type Integer) (MaxDepth :type Integer))
  (if (not (>= Depth MaxDepth))
    (bind (_block _exist) (`self.SpawnOrGetBlock` Coord Depth (`/Game/Paperland_DataTables/BFL_Database.GetBlockByType` "NewEnumerator6")))
    (if (not _exist)
      (for _array_element (`/Game/Paperland_Blueprints/GridSystem/BFL_GridSystem.GetNeighborCoordOffset`)
        (`self.GenerateBlocks` (`/Game/Paperland_Blueprints/GridSystem/BFL_GridSystem.OffsetCoord` _array_element (`local.Coord`)) (+ (`local.Depth`) 1) (`local.MaxDepth`))))))

(fn `GetNeighborBlocks`
  (params (Block :type "/Game/Paperland_Blueprints/Blocks/BP_Block Object Reference"))
  (returns (Neighbors :type "Array of /Game/Paperland_Blueprints/Blocks/BP_Block Object Reference"))
  (locals (NeighborBlocks :type "Array of /Game/Paperland_Blueprints/Blocks/BP_Block Object Reference"))
  (for _array_element (`/Game/Paperland_Blueprints/GridSystem/BFL_GridSystem.GetNeighborCoordOffset`)
    (bind (_value _returnvalue) (`BlueprintMapLibrary.Map_Find` (`self.BlockMap`) (`/Game/Paperland_Blueprints/GridSystem/BFL_GridSystem.OffsetCoord` _array_element (`/Game/Paperland_Blueprints/Blocks/BP_Block.Coord` (`local.Block`)))))
    (if _returnvalue
      (`KismetArrayLibrary.Array_Add` (`local.NeighborBlocks`) _value)))
  (return (`local.NeighborBlocks`)))

(fn `InitializeByConfig`
  (bind (_level _initblocks _sourceseablocks) (break `/Game/Paperland_DataTables/Config_Data/S_LevelConfig` (`self.Config`)))
  (for _array_element _sourceseablocks
    (`self.GenerateBlocks` _array_element 0 6)
    (bind (_keypin _valuepin) (`|MapForEach` _initblocks)
      (:`then`
        (`/Game/Paperland_Blueprints/Blocks/BPI_OceanInteraction.CreateTerrainBlock` _keypin (`/Game/Paperland_DataTables/BFL_Database.GetBlockByType` _valuepin))))))

(fn `SpawnBlock`
  (params (BlockInfo :type "/Game/Paperland_DataTables/Block_Data/S_BlockInfo Structure") (Coord :type "IntVector2 Structure") (Depth :type Integer))
  (returns (Block :type "/Game/Paperland_Blueprints/Blocks/BP_Block Object Reference"))
  (bind _returnvalue (`|SpawnActorFromClass` (`.Block_9_DC91E3CD466EA2992BB378A693657991` (break `/Game/Paperland_DataTables/Block_Data/S_BlockInfo` BlockInfo)) (`self.CoordToTransform` Coord) "Undefined" "MultiplyWithRoot" null (`local.Coord`) Depth (`local.BlockInfo`) null))
  (return _returnvalue))

(fn `SpawnOrGetBlock`
  (params (Coord :type "IntVector2 Structure") (Depth :type Integer) (BlockInfo :type "/Game/Paperland_DataTables/Block_Data/S_BlockInfo Structure"))
  (returns (Block :type "/Game/Paperland_Blueprints/Blocks/BP_Block Object Reference") (Exist :type Boolean))
  (bind _coord (`local.Coord`))
  (bind _depth (`local.Depth`))
  (bind (_value _returnvalue) (`BlueprintMapLibrary.Map_Find` (`self.BlockMap`) (`local.Coord`)))
  (if _returnvalue
    (if (< _depth (`/Game/Paperland_Blueprints/Blocks/BP_Block.RecursionDepth` _value))
      (set `/Game/Paperland_Blueprints/Blocks/BP_Block.RecursionDepth` _depth _value)
      (return _value false)
      (else
        (return _value true)))
    (else
      (bind _block (`self.SpawnBlock` BlockInfo _coord Depth))
      (`BlueprintMapLibrary.Map_Add` (`self.BlockMap`) _coord _block)
      (return _block false))))

(fn `SpawnTerrainBlock`
  (params (Coord :type "IntVector2 Structure") (BlockInfo :type "/Game/Paperland_DataTables/Block_Data/S_BlockInfo Structure"))
  (bind _blockmap (`self.BlockMap`))
  (bind (_value _returnvalue) (`BlueprintMapLibrary.Map_Find` _blockmap (`local.Coord`)))
  (if _returnvalue
    (bind _block (`self.SpawnBlock` BlockInfo (`local.Coord`) (`/Game/Paperland_Blueprints/Blocks/BP_Block.RecursionDepth` _value)))
    (`self.K2_DestroyActor` _value)
    (`BlueprintMapLibrary.Map_Add` _blockmap (`local.Coord`) _block)))

(fn `UserConstructionScript`)