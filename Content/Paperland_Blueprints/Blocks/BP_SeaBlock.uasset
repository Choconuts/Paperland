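; BP_SeaBlock is a clickable sea hex block in Paperland.
; Every tick it sets the Opacity material parameter on its SeaHex mesh, scaled by RecursionDepth relative to MaxDepth so higher depth values render more transparent.
; Clicking it calls CreateBlockTaskMessage on the game mode with itself as the block.
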(event `self.ReceiveTick`
  (params (DeltaSeconds :type "Float (single-precision)"))
  (`parent.ReceiveTick` DeltaSeconds)
  (`self.UpdateSeaColor`))

(event `self.ReceiveActorOnClicked`
  (params (ButtonPressed :type "Key Structure"))
  (`parent.ReceiveActorOnClicked` ButtonPressed)
  (message `/Game/Paperland_Blueprints/GameMode/BPI_Interaction.CreateBlockTask` (`GameplayStatics.GetGameMode`) self))

(fn `UpdateSeaColor`
  (`MeshComponent.SetScalarParameterValueOnMaterials` (`self.SeaHex`) "Opacity" (* (- 1.0 (/ (`self.RecursionDepth`) (`self.MaxDepth`))) 0.6)))

(fn `UserConstructionScript`
  (`parent.UserConstructionScript`))