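; GM_Paperland is the game mode for Paperland, handling level startup, block focus and task dialogs.
; On BeginPlay it spawns the ocean actor at the origin using the level config.
; FocusBlock events track a single focused block, switching its highlight when focus moves or clears.
; CreateBlockTask opens a terrain-creation dialog with hard-coded Chinese text asking for three same-colored cards, with Confirm initially disabled.
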(event `self.ReceiveBeginPlay`
  (`self.InitalizeOcean`))

(event `/Game/Paperland_Blueprints/GameMode/BPI_Interaction.FocusBlock`
  (params (Block :type "/Game/Paperland_Blueprints/Blocks/BP_Block Object Reference") (Focus :type Boolean))
  (`self.ChangeFocussedBlock` Block Focus))

(event `/Game/Paperland_Blueprints/GameMode/BPI_Interaction.CreateBlockTask`
  (params (SeaBlock :type "/Game/Paperland_Blueprints/Blocks/BP_SeaBlock Object Reference"))
  (`self.CreateTaskDialog`))

(fn `ChangeFocussedBlock`
  (params (Block :type "/Game/Paperland_Blueprints/Blocks/BP_Block Object Reference") (Focus :type Boolean))
  (if Focus
    (if (not (== Block (`self.FocussedBlock`)))
      (`self.UnfocusCurrentBlockIfNeeded`)
      (bind _output_get (set `self.FocussedBlock` (`local.Block`)))
      (`/Game/Paperland_Blueprints/Blocks/BP_BlockInteraction.HighlightBlock` _output_get "NewEnumerator1"))
    (else
      (`self.UnfocusCurrentBlockIfNeeded`))))

(fn `InitalizeOcean`
  (`|SpawnActorFromClass` "/Game/Paperland_Blueprints/Blocks/BP_Ocean.BP_Ocean_C" (`KismetMathLibrary.MakeTransform` (0.0 0.0 0.0)) "Undefined" "MultiplyWithRoot" (`GameplayStatics.GetPlayerController` 0) (`/Game/Paperland_DataTables/BFL_Database.GetLevelConfig` 0) null))

(fn `UnfocusCurrentBlockIfNeeded`
  (if (!= (`self.FocussedBlock`) null)
    (`/Game/Paperland_Blueprints/Blocks/BP_BlockInteraction.HighlightBlock` (`self.FocussedBlock`) "NewEnumerator0")
    (set `self.FocussedBlock` null)))

(fn `UserConstructionScript`
  (`parent.UserConstructionScript`))